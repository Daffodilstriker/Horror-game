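; BP_Paper is a paper prop that registers itself with the player character as an interactable.
; When an M-Charactor enters its Sphere, it stores that character, prints its name and sets the character's CurrentProp to itself.
; Leaving the sphere clears only the prop's stored reference, leaving the character's CurrentProp set.
; Its Oninterreact override just calls the parent implementation, so it adds no paper-specific behavior.
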(event OnComponentBeginOverlap(Sphere)
  (params (OverlappedComponent :type Primitive%20Component%20Object%20Reference) (OtherActor :type Actor%20Object%20Reference) (OtherComp :type Primitive%20Component%20Object%20Reference) (OtherBodyIndex :type Integer) (bFromSweep :type Boolean) (SweepResult :type Hit%20Result%20Structure%20%28by%20ref%29))
  (bind _asm_charactor (Utilities|Casting|CastToM-Charactor OtherActor))
  (bind _output_get (Variables|Default|SetCurrentInterract _asm_charactor))
  (Development|PrintString (Utilities|GetDisplayName _output_get))
  (Variables|/Game/GameCore/M-Player/M-Charactor.M-Charactor_C|SetCurrentProp _output_get self))

(event OnComponentEndOverlap(Sphere)
  (params (OverlappedComponent :type Primitive%20Component%20Object%20Reference) (OtherActor :type Actor%20Object%20Reference) (OtherComp :type Primitive%20Component%20Object%20Reference) (OtherBodyIndex :type Integer))
  (Utilities|Casting|CastToM-Charactor OtherActor)
  (Variables|Default|SetCurrentInterract 0))

(event EventBeginPlay)

(event Collision|EventActorBeginOverlap
  (params (OtherActor :type Actor%20Object%20Reference)))

(event EventTick
  (params (DeltaSeconds :type Float%20%28single-precision%29)))

(fn ConstructionScript)

(fn Oninterreact
  (|CallParentFunction))