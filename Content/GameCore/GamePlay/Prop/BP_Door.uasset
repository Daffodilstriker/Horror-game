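; BP_Door is an interactable door prop that opens only for a player holding a key.
; Box overlap registers the door as the character's CurrentProp and shows Widget1 if their PlayerState has the key; leaving hides both widgets.
; Oninterreact rechecks the key, then either fires DoorOpen once, swinging the yaw to 90 degrees by timeline, or shows the key-needed Widget.
; DoorClose plays a separate timeline without update logic and is not called here.
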(event OnComponentBeginOverlap(Box)
  (params (OverlappedComponent :type Primitive%20Component%20Object%20Reference) (OtherActor :type Actor%20Object%20Reference) (OtherComp :type Primitive%20Component%20Object%20Reference) (OtherBodyIndex :type Integer) (bFromSweep :type Boolean) (SweepResult :type Hit%20Result%20Structure%20%28by%20ref%29))
  (bind _asm_charactor (Utilities|Casting|CastToM-Charactor OtherActor))
  (bind _output_get (Variables|Default|SetCurrentInterract _asm_charactor))
  (Development|PrintString (Utilities|GetDisplayName _output_get))
  (Variables|/Game/GameCore/M-Player/M-Charactor.M-Charactor_C|SetCurrentProp _output_get self)
  (bind _asm_player_state (Utilities|Casting|CastToM-PlayerState (Variables|/Script/Engine.Pawn|GetPlayerState (Variables|Default|GetCurrentInterract))))
  (if (Variables|/Game/GameCore/M-Player/M-PlayerState.M-PlayerState_C|GetHoldingKey _asm_player_state)
    (Rendering|SetVisibility (Variables|Default|GetWidget1) true false)))

(event OnComponentEndOverlap(Box)
  (params (OverlappedComponent :type Primitive%20Component%20Object%20Reference) (OtherActor :type Actor%20Object%20Reference) (OtherComp :type Primitive%20Component%20Object%20Reference) (OtherBodyIndex :type Integer))
  (Utilities|Casting|CastToM-Charactor OtherActor)
  (Variables|Default|SetCurrentInterract 0)
  (Rendering|SetVisibility (Variables|Default|GetWidget) false false)
  (Rendering|SetVisibility (Variables|Default|GetWidget1) false false))

(event Custom|Door%20Close
  (Utilities|FlowControl|FlipFlop
    (:A
      (Timeline|Timeline Play))
    (:B
      (Timeline|Timeline ReverseFromEnd))))

(event Custom|Door%20Open
  (Utilities|FlowControl|FlipFlop
    (:A
      (bind _openprogress (Timeline|DoorOpen Play)
        (:Update
          (Transformation|SetRelativeRotation (Variables|Default|GetDoor) (Math|Rotator|MakeRotator 0.0 0.0 (Math|Float|MapRangeClamped _openprogress 0.0 1.0 0.0 9e+01)) false false))))
    (:B
      (Timeline|DoorOpen ReverseFromEnd))))

(event EventBeginPlay
  (Rendering|SetVisibility (Variables|Default|GetWidget) false false)
  (Rendering|SetVisibility (Variables|Default|GetWidget1) false false))

(event Collision|EventActorBeginOverlap
  (params (OtherActor :type Actor%20Object%20Reference)))

(event EventTick
  (params (DeltaSeconds :type Float%20%28single-precision%29)))

(fn ConstructionScript)

(fn Oninterreact
  (Utilities|IsValid (Variables|Default|GetCurrentInterract)
    (:Is%20Valid
      (bind _asm_player_state (Utilities|Casting|CastToM-PlayerState (Variables|/Script/Engine.Pawn|GetPlayerState (Variables|Default|GetCurrentInterract))))
      (if (Variables|/Game/GameCore/M-Player/M-PlayerState.M-PlayerState_C|GetHoldingKey _asm_player_state)
        (Utilities|FlowControl|DoOnce false
          (:Completed
            (CallFunction|DoorOpen)))
        (else
          (Development|PrintString "You have to find the key")
          (Rendering|SetVisibility (Variables|Default|GetWidget) true false))))
    (:Is%20Not%20Valid
      (Development|PrintString "Current Interract is none"))))