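; Vacuum cleaner Blueprint for the abandoned house that builds a bendable spline-shaped part, likely the hose, in its construction script.
; Each spline segment gets a collidable spline mesh using the configured static mesh and forward axis.
; An empty loop counts Spacing intervals along the spline, then its last index places one X-mirrored, collidable consumer electronic mesh at or near the spline's end.
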(fn ConstructionScript
  (bind _spline (Variables|Default|GetSpline))
  (bind _spline_2 (Variables|Default|GetSpline))
  (bind _spacing (Variables|Default|GetSpacing))
  (Utilities|FlowControl|Sequence
    (:then_0
      (for _index (range 0 (- (Spline|GetNumberOfSplinePoints _spline_2) 2))
        (bind _returnvalue (AddComponent|AddSplineMeshComponent false))
        (Components|StaticMesh|SetStaticMesh _returnvalue (Variables|Default|Getstatic%20mesh))
        (Rendering|Material|SetMaterial _spline_2 0 0)
        (SplineMesh|SetForwardAxis _returnvalue (Variables|Default|Getaxis) true)
        (Transformation|AttachComponentToComponent _returnvalue _spline_2 "" "KeepRelative" "KeepRelative" "KeepRelative" true)
        (SplineMesh|SetStartandEnd _returnvalue (Spline|GetLocationatSplinePoint _spline _index "Local") (Spline|GetTangentatSplinePoint _spline _index "Local") (Spline|GetLocationatSplinePoint _spline (+ _index 1 0) "Local") (Spline|GetTangentatSplinePoint _spline (+ _index 1 0) "Local") true :!class /Script/Engine.SplineMeshComponent)
        (Collision|SetCollisionEnabled _returnvalue "QueryAndPhysics")))
    (:then_1
      ;[1 1 1] Sigment of connect
      (for _index_2 (range 0 (.ReturnValue (Math|Float|Division(WholeandRemainder) (Spline|GetSplineLength _spline_2) _spacing)))
        _))
    (:then_2
      (bind _returnvalue_2 (AddComponent|AddStaticMeshComponent false (Math|Transform|MakeTransform (Spline|GetLocationatDistanceAlongSpline _spline_2 (* _index_2 _spacing) "Local") (Spline|GetRotationatDistanceAlongSpline _spline_2 (* _index_2 _spacing) "Local") "-1.000000,1.000000,1.000000")))
      (Components|StaticMesh|SetStaticMesh _returnvalue_2 "/Game/Abandoned_house/Meshes/house_props/consumer_electronics/SM_consumer_electronic_5_2.SM_consumer_electronic_5_2")
      (Collision|SetCollisionEnabled _returnvalue_2 "QueryAndPhysics"))))